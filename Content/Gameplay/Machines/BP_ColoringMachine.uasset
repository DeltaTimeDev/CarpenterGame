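; BP_ColoringMachine is a machine actor that straightens products entering its painting area and provides paint feedback.
; On overlap, the authority runs a timeline that lerps the ProductActor's current rotation toward zero.
; A separate PaintEffect event, not called within this graph, spawns confetti tinted by the given color and plays a blob sound at the painting area.
; The color change on the product itself is not handled here.
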(event `self.PaintingArea.OnComponentBeginOverlap`
  (params (OverlappedComponent :type "PrimitiveComponent Object Reference") (OtherActor :type "Actor Object Reference") (OtherComp :type "PrimitiveComponent Object Reference") (OtherBodyIndex :type Integer) (bFromSweep :type Boolean) (SweepResult :type "HitResult Structure (by ref)"))
  (`self.RotationAnim` OtherActor))

(event `RotationAnim`
  (params (Actor :type "Actor Object Reference"))
  ; Rotation Anim
  (`/Engine/EditorBlueprintResources/ActorMacros.Switch Has Authority`
    (:`Authority`
      (bind _asproduct_actor (cast `ProductActor` Actor))
      (bind (_direction _rotationamount) (`Timeline|Timeline` :!via `PlayFromStart`)
        (:`Update`
          (`self.K2_SetActorRotation` _asproduct_actor (`KismetMathLibrary.RLerp` (`self.K2_GetActorRotation` _asproduct_actor) (struct) _rotationamount) false))))))

(event `self.PaintEffect`
  (params (Color :type "LinearColor Structure"))
  (bind _returnvalue (`SceneComponent.K2_GetComponentLocation` (`self.PaintingArea`)))
  ; Paint Visual Effect
  (bind _returnvalue_2 (`NiagaraFunctionLibrary.SpawnSystemAtLocation` "/Game/Effects/ConffetiEffect.ConffetiEffect" _returnvalue))
  (`NiagaraComponent.SetVariableLinearColor` _returnvalue_2 "PaintColor" Color)
  ; Paint Visual Effect
  (`GameplayStatics.PlaySoundAtLocation` "/Game/Sounds/Blob.Blob" _returnvalue (struct) 1.0 1.0 0.0 null null null null))

(fn `UserConstructionScript`)